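; BP_Claws is a concrete action that deals a claw attack to a target and rewards the caster with a crit buff.
; It overrides ApplyActionStrategy, running the parent check first and failing if that fails or the target has the Block status.
; Otherwise it damages the target through its health component, applies BP_CritBuffStatus to the caster and reports success.
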(fn ApplyActionStrategy
  (params (ActionTarget :type Turn%20Based%20Actor%20Object%20Reference) (ActionCaster :type Turn%20Based%20Actor%20Object%20Reference))
  (bind _returnvalue (|CallParentFunction ActionTarget ActionCaster))
  (if _returnvalue
    (if (Class|StatusComponent|HasStatus (Class|TurnBasedActor|GetStatusComponent ActionTarget) "ST_Block")
      (return false)
      (else
        (Class|HealthComponent|TakeDamage (Class|TurnBasedActor|GetHealthComponent ActionTarget) (Variables|Default|GetDamage))
        (Class|StatusSolver|ApplyStatus (Utilities|Struct|MakeApplyStatusContext "/Game/Blueprint/Logic/Status/BP_CritBuffStatus.BP_CritBuffStatus_C" ActionCaster))
        (return true)))
    (else
      (return false))))