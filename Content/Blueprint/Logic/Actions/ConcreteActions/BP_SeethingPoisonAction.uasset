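; BP_SeethingPoisonAction is an action strategy that damages a target harder the more Poison statuses it carries.
; ApplyActionStrategy runs the parent check first, then fails without damage if the target has a Block status.
; Otherwise it calls TakeDamage on the target's health component twice: once for base Damage, once for Damage multiplied by the applied Poison count.
; It returns whether the action landed.
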(fn ApplyActionStrategy
  (params (ActionTarget :type Turn%20Based%20Actor%20Object%20Reference) (ActionCaster :type Turn%20Based%20Actor%20Object%20Reference))
  (bind _returnvalue (Class|TurnBasedActor|GetHealthComponent ActionTarget))
  (bind _returnvalue_2 (|CallParentFunction ActionTarget ActionCaster))
  (if _returnvalue_2
    (if (Class|StatusComponent|HasStatus (Class|TurnBasedActor|GetStatusComponent ActionTarget) "ST_Block")
      (return false)
      (else
        (Class|HealthComponent|TakeDamage _returnvalue (Variables|Default|GetDamage))
        (Class|HealthComponent|TakeDamage _returnvalue (* (Utilities|Array|Length (Class|StatusComponent|GetAllAppliedStatusbyEnum (Class|TurnBasedActor|GetStatusComponent ActionTarget) "ST_Poison")) (Variables|Default|GetDamage)))
        (return true)))
    (else
      (return false))))