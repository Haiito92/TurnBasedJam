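; Psychic Horror Evocation is a combat action that deals damage to a target at a health cost to the caster.
; After the parent strategy succeeds, a Block status on the target makes the action fail.
; Otherwise the caster takes a fraction of the final damage as recoil, and the target takes all of it unless Confused.
; Final damage rolls for a critical multiplier, with odds rising per CritBuff stack on the caster.
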(fn ApplyActionStrategy
  (params (ActionTarget :type Turn%20Based%20Actor%20Object%20Reference) (ActionCaster :type Turn%20Based%20Actor%20Object%20Reference))
  (bind _returnvalue (|CallParentFunction ActionTarget ActionCaster))
  (if _returnvalue
    (if (Class|StatusComponent|HasStatus (Class|TurnBasedActor|GetStatusComponent ActionTarget) "ST_Block")
      (return false)
      (else
        (bind _output_get (LocalVariables|SetFinalDamage (CallFunction|CalculateFinalDamage ActionCaster)))
        (Class|HealthComponent|TakeDamage (Class|TurnBasedActor|GetHealthComponent ActionCaster) (* _output_get 0.1))
        (if (Class|StatusComponent|HasStatus (Class|TurnBasedActor|GetStatusComponent ActionTarget) "ST_Confused")
          _
          (else
            (Class|HealthComponent|TakeDamage (Class|TurnBasedActor|GetHealthComponent ActionTarget) (LocalVariables|GetFinalDamage))))
        (return true)))
    (else
      (return false))))

(fn CalculateFinalDamage
  (params (ActionCaster :type Turn%20Based%20Actor%20Object%20Reference))
  (bind _damage (Variables|Default|GetDamage))
  (return (Math|Float|SelectFloat (* (Variables|Default|GetCritMultiplicator) _damage) _damage (<= (Math|Random|RandomFloatinRange 0.0 1.0) (Math|Float|Clamp(Float) (* (Utilities|Array|Length (Class|StatusComponent|GetAllAppliedStatusbyEnum (Class|TurnBasedActor|GetStatusComponent ActionCaster) "ST_CritBuff")) (Math|Float|MakeLiteralFloat 0.2)))))))