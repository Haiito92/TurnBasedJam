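; BP_BiteAction is a concrete action that applies bite damage to a target.
; It overrides ApplyActionStrategy and continues only if the parent implementation succeeds.
; A Block status on the target's status component negates the bite, printing a warning and returning false.
; Otherwise it passes the damage value from its Data to the target's health component and returns true.
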(fn ApplyActionStrategy
  (params (ActionTarget :type Turn%20Based%20Actor%20Object%20Reference))
  (bind _returnvalue (|CallParentFunction ActionTarget))
  (if _returnvalue
    (if (Class|StatusComponent|HasStatus (Class|TurnBasedActor|GetStatusComponent ActionTarget) "ST_Block")
      (Class|TurnBasedDebugLibrary|Print "Warning" "[BP_BiteAction]  Blocked!" 3.0)
      (return false)
      (else
        (Class|HealthComponent|TakeDamage (Class|TurnBasedActor|GetHealthComponent ActionTarget) (Variables|/Script/TurnBasedJam.ActionData|GetDamage (Variables|Default|GetData)))
        (return true)))
    (else
      (return false))))