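; Test Blueprint that previews hero and vampire combat animations and status effects on one static mesh.
; Material parameters switch character, sprite frame and status look, while VFX components play the effect and Timelines drive Y movement and hit tint.
; Only the hero confusion preview runs on BeginPlay.
; The block, hit, poison and vampire attack sequences sit disconnected from any event.
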(event EventBeginPlay
  ;[0.15 0.15 0.15 0.5] HeroConfusedPoison
  (Rendering|Material|SetScalarParameterValueonMaterials (Variables|Default|GetStaticMesh) "CharacterSwitch" 0.0)
  (Components|Activation|Activate (Variables|Default|GetVFX_Status_Confusion) true)
  (Rendering|Material|SetScalarParameterValueonMaterials (Variables|Default|GetStaticMesh) "Confused" 1.0))

(fn ConstructionScript)